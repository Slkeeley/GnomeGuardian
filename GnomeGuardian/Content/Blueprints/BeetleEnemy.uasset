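; Beetle enemy Blueprint that chases the player once pawn sensing spots a pawn.
; OnSeePawn latches SeesPlayer, and Tick then calls FollowsPlayer every frame to issue an AI move toward player 0.
; On arrival it toggles a CanAttack cooldown around a delay, but no attack is implemented and each follow call re-enables the flag.
; A self-repeating random-point patrol exists in MoveAI, but BeginPlay is empty and nothing starts it.
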(event `MoveAI`
  ;[1 1 1] Patrol
  (bind _output_get (set `self.Random Location` (`NavigationSystemV1.K2_GetRandomReachablePointInRadius` (`self.K2_GetActorLocation`) 1000.0 null null)))
  (`|AIMoveTo` self _output_get null
    (:`then`
      (`KismetSystemLibrary.Delay` 3.0)
      (`self.MoveAI`))
    (:`OnFail`
      (`KismetSystemLibrary.Delay` 0.2)
      (`self.MoveAI`))))

(event `self.ReceiveBeginPlay`
  ;[1 1 1] Random Movement
)

(event `self.ReceiveTick`
  (params (DeltaSeconds :type "Float (single-precision)"))
  (if (`self.seesPlayer`)
    (`self.Follows Player`)))

(event `self.PawnSensing.OnSeePawn`
  (params (Pawn :type "Pawn Object Reference"))
  ;[1 1 1] Move To Player
  (set `self.seesPlayer` true)
  (`self.Follows Player`))

(event `Follows Player`
  ;[1 1 1] Move To Player
  (set `self.canAttack` true)
  (if (`self.seesPlayer`)
    (`|AIMoveTo` self (0.0 0.0 0.0) (`GameplayStatics.GetPlayerCharacter` 0) 50.0
      (:`OnSuccess`
        (if (`self.canAttack`)
          (set `self.canAttack` false)
          (`KismetSystemLibrary.Delay` 2.0)
          (set `self.canAttack` true))))))

(fn `UserConstructionScript`)