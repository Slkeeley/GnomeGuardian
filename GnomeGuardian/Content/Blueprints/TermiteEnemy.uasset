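; Termite enemy that detects pawns through PawnSensing, loses health from any damage and destroys itself at zero health, checked on Tick.
; Seeing a pawn sets a flag and calls FollowsPlayer, then MoveAI after a retriggerable delay; neither function is defined here.
; An AIMoveTo chase with a cooldown-gated melee attack is present but unconnected, so it never runs.
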(event `self.PawnSensing.OnSeePawn`
  (params (Pawn :type "Pawn Object Reference"))
  ;[1 1 1] Move To Player
  (`|ExecutionSequence`
    (:`then_0`
      (set `self.seesPlayer` true)
      (`self.Follows Player`))
    (:`then_1`
      (`KismetSystemLibrary.RetriggerableDelay` 1.0)
      (`self.MoveAI`))))

(event `self.ReceiveTick`
  (params (DeltaSeconds :type "Float (single-precision)"))
  ;[1 1 1] Take Damage
  (if (<= (`self.Health`) 0.0)
    (`self.K2_DestroyActor`)))

(event `self.ReceiveAnyDamage`
  (params (Damage :type "Float (single-precision)") (DamageType :type "DamageType Object Reference") (InstigatedBy :type "Controller Object Reference") (DamageCauser :type "Actor Object Reference"))
  ;[1 1 1] Take Damage
  (set `self.Health` (- (`self.Health`) Damage)))

(fn `UserConstructionScript`
  (`parent.UserConstructionScript`))